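; Pickup actor Blueprint, built on a C++ parent, that plays a short spin effect when collected and then removes itself.
; The Collected event is guarded by a DoOnce and calls the parent's C++ implementation first.
; It then sharply increases the RotatingMovement component's roll and yaw rates and destroys the actor after a one-second delay.
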(event EventBeginPlay)

(event Collision|EventActorBeginOverlap
  (params (OtherActor :type Actor%20Object%20Reference)))

(event EventTick
  (params (DeltaSeconds :type Float%20%28single-precision%29)))

(event EventCollected
  ;[1 1 1] Pickup Action
  (Utilities|FlowControl|DoOnce false
    (:Completed
      (|CallParentFunction) ; Calls Collected function implemented in CPP
      (Variables|/Script/Engine.RotatingMovementComponent|SetRotationRate (Variables|Default|GetRotatingMovement) (Math|Rotator|MakeRotator (* (+ (.roll (Variables|/Script/Engine.RotatingMovementComponent|GetRotationRate (Variables|Default|GetRotatingMovement))) 9e+01) 1e+01) 0.0 (* (.yaw (Variables|/Script/Engine.RotatingMovementComponent|GetRotationRate (Variables|Default|GetRotatingMovement))) 1e+01)))
      (Utilities|FlowControl|Delay 1.0)
      (Actor|DestroyActor))))

(fn ConstructionScript)